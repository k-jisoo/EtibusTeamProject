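; Main player controller Blueprint that relays player skill, stat and gold updates to the skill shop UI.
; Each update event casts SkillShopWidget to SkillStoreWidget and calls the matching refresh function for skill slots, inventory, enhancement items, stats or gold.
; Max HP, max MP, power and speed are truncated to integers before display.
; Current HP changes are only printed to screen and never reach the widget.
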(event EventBeginPlay)

(event EventTick
  (params (DeltaSeconds :type Float%20%28single-precision%29)))

(event EventOnUpdateMyCurHp
  (params (CurHp :type Float%20%28single-precision%29) (MaxHp :type Float%20%28single-precision%29))
  (Development|PrintString (Utilities|String|ToString(Float) CurHp)))

(event EventOnUpdateSkills
  (params (skillDatas :type Array%20of%20Skill%20Base%20Object%20References))
  (bind _asskill_store_widget (Utilities|Casting|CastToSkillStoreWidget (Variables|Default|GetSkillShopWidget)))
  (Default|UpdateSkillSlot _asskill_store_widget skillDatas))

(event EventOnUpdateEnhancementObjs
  (params (objDatas :type Array%20of%20Stat%20Enhancement%20Object%20Base%20Object%20References))
  (bind _asskill_store_widget (Utilities|Casting|CastToSkillStoreWidget (Variables|Default|GetSkillShopWidget)))
  (Default|UpdateEnhancementItem _asskill_store_widget objDatas))

(event EventOnUpdateMySkillLevel
  (params (skillDatas :type Array%20of%20Skill%20Base%20Object%20References))
  (bind _asskill_store_widget (Utilities|Casting|CastToSkillStoreWidget (Variables|Default|GetSkillShopWidget)))
  (Default|UpdateInvenSlot _asskill_store_widget skillDatas))

(event EventOnUpdateMyMaxHp
  (params (CurHp :type Float%20%28single-precision%29) (MaxHp :type Float%20%28single-precision%29))
  (bind _asskill_store_widget (Utilities|Casting|CastToSkillStoreWidget (Variables|Default|GetSkillShopWidget)))
  (Default|UpdateHp _asskill_store_widget (Math|Float|Truncate MaxHp)))

(event EventOnUpdateMyMaxMp
  (params (CurMp :type Float%20%28single-precision%29) (MaxMp :type Float%20%28single-precision%29))
  (bind _asskill_store_widget (Utilities|Casting|CastToSkillStoreWidget (Variables|Default|GetSkillShopWidget)))
  (Default|UpdateMp _asskill_store_widget (Math|Float|Truncate MaxMp)))

(event EventOnUpdateMyPower
  (params (Power :type Float%20%28single-precision%29))
  (bind _asskill_store_widget (Utilities|Casting|CastToSkillStoreWidget (Variables|Default|GetSkillShopWidget)))
  (Default|UpdatePower _asskill_store_widget (Math|Float|Truncate Power)))

(event EventOnUpdateMySpeed
  (params (Speed :type Float%20%28single-precision%29))
  (bind _asskill_store_widget (Utilities|Casting|CastToSkillStoreWidget (Variables|Default|GetSkillShopWidget)))
  (Default|UpdateSpeed _asskill_store_widget (Math|Float|Truncate Speed)))

(event EventOnUpdateMyGold
  (params (coin :type Integer))
  (bind _asskill_store_widget (Utilities|Casting|CastToSkillStoreWidget (Variables|Default|GetSkillShopWidget)))
  (Default|UpdateGold _asskill_store_widget coin))

(fn ConstructionScript)